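; Gameplay cue for the hero's magic shield, providing its sound and visual effect while the cue is active.
; WhileActive plays the activation sound at the target's location and spawns a Niagara shield system attached to the cue's target attach component at MagicShieldSocket.
; It stores the spawned system so OnRemove can destroy the component, if still valid, when the cue ends.
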(fn `OnRemove`
  (params (MyTarget :type "Actor Object Reference") (Parameters :type "GameplayCueParameters Structure (by ref)"))
  (returns (ReturnValue :type Boolean))
  (bind _spawnedmagicshieldsystem (`self.SpawnedMagicShieldSystem`)
    (:`then`
      (`ActorComponent.K2_DestroyComponent` _spawnedmagicshieldsystem null)
      (return false))
    (:`else`)))

(fn `UserConstructionScript`)

(fn `WhileActive`
  (params (MyTarget :type "Actor Object Reference") (Parameters :type "GameplayCueParameters Structure (by ref)"))
  (returns (ReturnValue :type Boolean))
  (`|ExecutionSequence`
    (:`then_0`
      (`GameplayStatics.PlaySoundAtLocation` null "/Game/Assets/Sounds/Weapons/Block/SC_MagicShieldActiavte.SC_MagicShieldActiavte" (`self.K2_GetActorLocation` (`local.MyTarget`)) (struct) 1.0 1.0 0.0 null null null null))
    (:`then_1`
      (bind _returnvalue (`NiagaraFunctionLibrary.SpawnSystemAttached` "/Game/Assets/Niagara/Shield/NS_Shield_1.NS_Shield_1" (`.TargetAttachComponent` (`AbilitySystemBlueprintLibrary.BreakGameplayCueParameters` Parameters)) "MagicShieldSocket" (0.0 0.0 0.0) (struct) "KeepRelativeOffset"))
      (set `self.SpawnedMagicShieldSystem` _returnvalue)
      (return false))))