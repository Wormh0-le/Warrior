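; GC_Hero_PerfectBlock is a gameplay cue that plays the visual burst for a hero's perfect block.
; On execute, it spawns the NS_RefractionBurst system slightly in front of the MagicShieldSocket on the cue's target attach component, oriented along the target actor's forward vector.
; It then returns the result of the parent OnExecute.
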(fn `OnExecute`
  (params (MyTarget :type "Actor Object Reference") (Parameters :type "GameplayCueParameters Structure (by ref)"))
  (returns (ReturnValue :type Boolean))
  (bind _returnvalue (`Actor.GetActorForwardVector` (`local.MyTarget`)))
  (`NiagaraFunctionLibrary.SpawnSystemAtLocation` null "/Game/Assets/Niagara/Refraction/NS_RefractionBurst.NS_RefractionBurst" (+ (* _returnvalue 30.0) (`SceneComponent.GetSocketLocation` (`.TargetAttachComponent` (`AbilitySystemBlueprintLibrary.BreakGameplayCueParameters` (`local.Parameters`))) "MagicShieldSocket")) (`KismetMathLibrary.MakeRotFromX` _returnvalue))
  (return (`parent.OnExecute` (`local.MyTarget`) (`local.Parameters`))))