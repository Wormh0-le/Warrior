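; GC_Enemy_AttackWarning is a gameplay cue that shows a Niagara warning effect, apparently for an enemy's unblockable attack.
; On execute, it spawns the system in front of the target's eye viewpoint, offset along the actor's forward vector by the cue's RawMagnitude and facing that direction.
; It then attaches the effect to the target's root component with KeepRelative rules and calls the parent implementation.
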(fn `OnExecute`
  (params (MyTarget :type "Actor Object Reference") (Parameters :type "GameplayCueParameters Structure (by ref)"))
  (returns (ReturnValue :type Boolean))
  (bind _returnvalue (`Actor.GetActorForwardVector` MyTarget))
  (bind _returnvalue_2 (`NiagaraFunctionLibrary.SpawnSystemAtLocation` null "/Game/Assets/Niagara/Warning/NS_UnbloackableWarning.NS_UnbloackableWarning" (+ (`Actor.GetActorEyesViewPoint` MyTarget) (* _returnvalue (`.RawMagnitude` (`AbilitySystemBlueprintLibrary.BreakGameplayCueParameters` Parameters)))) (`KismetMathLibrary.Conv_VectorToRotator` _returnvalue)))
  (`SceneComponent.K2_AttachToComponent` _returnvalue_2 (`Actor.RootComponent` (`local.MyTarget`)) "None" "KeepRelative" "KeepRelative" "KeepRelative" true)
  (return (`parent.OnExecute` (`local.MyTarget`) (`local.Parameters`))))