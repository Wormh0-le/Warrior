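; Survival game mode Blueprint that presents the progress of wave-based play on screen.
; On BeginPlay it binds to the survival state-change delegate and adds a WBP_WaveInfo widget to the viewport.
; Each wave state sets the widget's text, then either starts a countdown or chains fade-in and fade-out animations, labeling the last wave as final.
; All-waves-done and player-death states only print screen messages.
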(event `self.ReceiveBeginPlay`
  (add `self.OnSurvivalGameModeStateChanged` (delegate `OnSurvivalGameModeStateChanged_Event`))
  (`self.CreateWaveInfoWidget`))

(event `OnSurvivalGameModeStateChanged_Event` :!signature `self.OnSurvivalGameModeStateChanged`
  (params (CurrentState :type "EWarriorSurvivalGameModeState Enum" :default "WaitSpawnNewWave"))
  (bind _waveinfowidget (`self.WaveInfoWidget`))
  (bind _waveinfowidget_2 (`self.WaveInfoWidget`))
  (bind _waveinfowidget_3 (`self.WaveInfoWidget`))
  (bind _waveinfowidget_4 (`self.WaveInfoWidget`))
  (bind _waveinfowidget_5 (`self.WaveInfoWidget`))
  (bind _waveinfowidget_6 (`self.WaveInfoWidget`))
  (bind _currentwave (`self.CurrentWave`))
  (bind _tb_waveinfotext (`/Game/Blueprints/Widgets/Hero/WBP_WaveInfo.TB_WaveInfoText` (`self.WaveInfoWidget`)))
  (switch `EWarriorSurvivalGameModeState` CurrentState
    (:`WaitSpawnNewWave`
      ;[0.6615 0.7436 0.974] Wait Spawn New Wave
      (`TextBlock.SetText` (`/Game/Blueprints/Widgets/Hero/WBP_WaveInfo.TB_WaveInfoText` _waveinfowidget_6) "New Wave Coming In:")
      (`Widget.SetVisibility` _waveinfowidget_6 "Visible")
      (`UserWidget.PlayAnimation` _waveinfowidget_6 (`/Game/Blueprints/Widgets/Hero/WBP_WaveInfo.WaveFadeInAnimation` _waveinfowidget_6) 0.0 1 "Forward" 1.0 false)
      (`/Game/Blueprints/Widgets/Hero/WBP_WaveInfo.StartCountdown` _waveinfowidget_6 (`self.SpawnNewWaveWaitTime`)))
    (:`SpawningNewWave`
      ;[0.5236 0.5885 0.7708] Spawning
      (if (== (`self.TotalWavesToSpawn`) _currentwave)
        (`TextBlock.SetText` _tb_waveinfotext (`|FormatText` "Final Wave"))
        (else
          (`TextBlock.SetText` _tb_waveinfotext (`|FormatText` "Wave {CurrentWave}" _currentwave))))
      (`|PlayAnimation2` _waveinfowidget_2 (`/Game/Blueprints/Widgets/Hero/WBP_WaveInfo.WaveFadeInAnimation` _waveinfowidget_2)
        (:`Finished`
          (`|PlayAnimation2` _waveinfowidget_4 (`/Game/Blueprints/Widgets/Hero/WBP_WaveInfo.WaveFadeOutAnimation` _waveinfowidget_4)
            (:`Finished`
              (`Widget.SetVisibility` _waveinfowidget_5 "Hidden")
              (`Widget.SetRenderOpacity` _waveinfowidget_5 1.0))))))
    (:`WaveCompleted`
      ;[0.4316 0.4851 0.6354] Spawn Wave Completed
      (`TextBlock.SetText` (`/Game/Blueprints/Widgets/Hero/WBP_WaveInfo.TB_WaveInfoText` _waveinfowidget) (`|FormatText` "Wave {CurrentWave} Completed" (`self.CurrentWave`)))
      (`Widget.SetVisibility` _waveinfowidget "Visible")
      (`UserWidget.PlayAnimation` _waveinfowidget_3 (`/Game/Blueprints/Widgets/Hero/WBP_WaveInfo.WaveFadeInAnimation` _waveinfowidget_3) 0.0 1 "Forward" 1.0 false)
      (`/Game/Blueprints/Widgets/Hero/WBP_WaveInfo.StartCountdown` _waveinfowidget_3 (`self.WaveCompletedWaitTime`)))
    (:`AllWavesDone`
      (`KismetSystemLibrary.PrintString` "All Wave Completed" true true (struct :`G` 0.66 :`B` 1.0 :`A` 1.0) 8.0))
    (:`PlayerDied`
      (`KismetSystemLibrary.PrintString` "You Died" true true (struct :`R` 1.0 :`A` 1.0) 10.0))))

(fn `CreateWaveInfoWidget`
  (bind _returnvalue (`|CreateWidget` "/Game/Blueprints/Widgets/Hero/WBP_WaveInfo.WBP_WaveInfo_C"))
  (set `self.WaveInfoWidget` _returnvalue)
  (`UserWidget.AddToViewport` _returnvalue 0))

(fn `UserConstructionScript`)